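; BP_PereTuto is the tutorial father AI character, handling its footstep audio and its own removal.
; Each Tick it destroys itself if CanDestroy is set, otherwise it reads MaxWalkSpeed as the movement state.
; Zero stops FootStepsDad, exactly 300 starts it at walking pitch, and higher speeds start it at a faster pitch.
; A playing flag prevents restarts, so pitch only changes after a stop.
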(event `self.ReceiveTick`
  (params (DeltaSeconds :type "Float (single-precision)"))
  (bind _footstepsdad (`self.FootStepsDad`))
  (bind _footstepsplaying (`self.FootStepsPlaying`))
  ;[0 0.6771 1] FootstepsDad
  (if (`self.CanDestroy`)
    (`self.K2_DestroyActor`)
    (else
      (`/Engine/EditorBlueprintResources/StandardMacros.CompareFloat` (`CharacterMovementComponent.MaxWalkSpeed` (`self.CharacterMovement`))
        (:`>`
          (`/Engine/EditorBlueprintResources/StandardMacros.CompareFloat` (`CharacterMovementComponent.MaxWalkSpeed` (`self.CharacterMovement`)) 300.0
            (:`>`
              (if (not _footstepsplaying)
                (`AudioComponent.SetPitchMultiplier` _footstepsdad 2.0)
                (`AudioComponent.Play` _footstepsdad 0.0)
                (set `self.FootStepsPlaying` true)))
            (:`==`
              (if (not _footstepsplaying)
                (`AudioComponent.SetPitchMultiplier` _footstepsdad 1.2)
                (`AudioComponent.Play` _footstepsdad 0.0)
                (set `self.FootStepsPlaying` true)))))
        (:`==`
          (set `self.FootStepsPlaying` false)
          (`AudioComponent.Stop` (`self.FootStepsDad`)))))))

(fn `UserConstructionScript`)